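; BP_GameController runs a projectile launcher game through Ready, Aiming, Powering and Fly stages, broadcasting each change.
; On BeginPlay it creates the game UI and finds the level's BP_Projectile.
; Each AdvanceStage call moves forward: one timeline sweeps the launch angle, another fills the power bar, then the sampled power scales a physics impulse along the projectile's local up axis.
; GameRestart restores Ready and resets the projectile's transform and physics.
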(event `self.ReceiveBeginPlay`
  (set `self.GameStage` "NewEnumerator0")
  (`KismetSystemLibrary.PrintString` "遊戲階段設為 \"等待按下按鈕\"")
  (bind _returnvalue (`|CreateWidget` "/Game/AsiaDemoLauncherGame/UI/WBP_GameUI.WBP_GameUI_C"))
  (`|ExecutionSequence`
    (:`then_0`
      (`UserWidget.AddToViewport` _returnvalue 0)
      (`self.OnGameStageChange`)
      (bind _returnvalue_2 (`GameplayStatics.GetActorOfClass` "/Game/AsiaDemoLauncherGame/Blueprints/Actor/BP_Projectile.BP_Projectile_C"))
      (set `self.Projectile` _returnvalue_2))
    (:`then_1`
      (set `self.GameUI` _returnvalue))))

(event `AdvanceStage`
  (bind _projectile (`self.Projectile`))
  (bind _sphere (`/Game/AsiaDemoLauncherGame/Blueprints/Actor/BP_Projectile.Sphere` _projectile))
  (`KismetSystemLibrary.PrintString` "觸發改變遊戲階段事件")
  (switch `/Game/AsiaDemoLauncherGame/Blueprints/Actor/E_GameStage` (`self.GameStage`)
    (:`NewEnumerator0`
      (set `self.GameStage` "NewEnumerator1")
      (`KismetSystemLibrary.PrintString` "遊戲狀態改變為瞄準階段")
      (`self.OnGameStageChange`)
      (bind (_direction _angletrack) (`Timeline|Timeline` :!label _label)
        (:`Update`
          (bind _returnvalue (`KismetMathLibrary.Lerp` 15.0 75.0 _angletrack))
          (set `self.ShootAngle` _returnvalue)
          (`self.K2_SetActorRotation` (`self.Projectile`) (`KismetMathLibrary.MakeRotator` _returnvalue) false))))
    (:`NewEnumerator1`
      (set `self.GameStage` "NewEnumerator2")
      (`KismetSystemLibrary.PrintString` "遊戲階段改變為蓄力階段")
      (`self.OnGameStageChange`)
      (`|ExecutionSequence`
        (:`then_0`
          (goto _label :!via `Stop`))
        (:`then_1`
          (`KismetSystemLibrary.PrintString` "Hello")
          (bind (_direction_2 _angletrack_2) (`Timeline|Timeline_0` :!label _label_2)
            (:`Update`
              (set `ProgressBar.Percent` _angletrack_2 (`/Game/AsiaDemoLauncherGame/UI/WBP_GameUI.Bar_Power` (`self.GameUI`))))))))
    (:`NewEnumerator2`
      (set `self.GameStage` "NewEnumerator3")
      (`KismetSystemLibrary.PrintString` "遊戲階段改變為發射階段")
      (`self.OnGameStageChange`)
      (`|ExecutionSequence`
        (:`then_0`
          (goto _label_2 :!via `Stop`))
        (:`then_1`
          (bind _output_get (set `self.Power` _angletrack_2))
          (`PrimitiveComponent.SetSimulatePhysics` _sphere true)
          (`PrimitiveComponent.AddImpulse` _sphere (* (* _output_get 1000.0) (`KismetMathLibrary.TransformDirection` (`self.GetTransform` _projectile) (`KismetMathLibrary.MakeVector` 0.0 0.0 1.0))) "None" true))))))

(event `GameRestart`
  (bind _projectile (`self.Projectile`))
  (`|ExecutionSequence`
    (:`then_0`
      (set `self.GameStage` "NewEnumerator0"))
    (:`then_1`
      (`SceneComponent.K2_SetWorldLocationAndRotation` (`Actor.RootComponent` _projectile) (200.0 0.0 80.0) (struct :`Roll` 15.0) false false)
      (`PrimitiveComponent.SetSimulatePhysics` (`/Game/AsiaDemoLauncherGame/Blueprints/Actor/BP_Projectile.Sphere` _projectile) false))
    (:`then_2`
      (`self.OnGameStageChange`))))

(fn `UserConstructionScript`)